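; BP_InteractiveCube_FuzeBtn is a cube that gives color feedback for gaze-based fuse interaction.
; It creates a dynamic material on BeginPlay and sets ColorParam yellow on hover, white on exit and green on trigger.
; After a trigger, RecentlyTriggered blocks hover and exit changes until a retriggerable delay restores white, guarding a race when gaze leaves as the fuse fires.
; The BillboardUpdate helper for the text render is never executed.
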(event EventOnGazeHover
  (if (not (Variables|Default|GetRecentlyTriggered))
    (Rendering|Material|SetVectorParameterValue (Variables|Default|GetDinamicMaterial) "ColorParam" "(R=1.000000,G=1.000000,B=0.000000,A=1.000000)" :!class /Script/Engine.MaterialInstanceDynamic)))

(event Collision|EventActorBeginOverlap
  (params (OtherActor :type Actor%20Object%20Reference)))

(event EventOnGazeExit
  (if (not (Variables|Default|GetRecentlyTriggered))
    (Rendering|Material|SetVectorParameterValue (Variables|Default|GetDinamicMaterial) "ColorParam" "(R=1.000000,G=1.000000,B=1.000000,A=1.000000)" :!class /Script/Engine.MaterialInstanceDynamic)))

(event EventTick
  (params (DeltaSeconds :type Float%20%28single-precision%29)))

(event EventOnFuseTriggered
  (Rendering|Material|SetVectorParameterValue (Variables|Default|GetDinamicMaterial) "ColorParam" "(R=0.000000,G=1.000000,B=0.000000,A=1.000000)" :!class /Script/Engine.MaterialInstanceDynamic)
  (Variables|Default|SetRecentlyTriggered true)
  (Utilities|FlowControl|RetriggerableDelay 0.5)
  ;[1 1 1] Necesario por condicion de carrera al quitar la vista del cubo justo cuando salta el evento
  (Rendering|Material|SetVectorParameterValue (Variables|Default|GetDinamicMaterial) "ColorParam" "(R=1.000000,G=1.000000,B=1.000000,A=1.000000)" :!class /Script/Engine.MaterialInstanceDynamic)
  (Variables|Default|SetRecentlyTriggered false))

(event EventBeginPlay
  (bind _returnvalue (Rendering|Material|CreateDynamicMaterialInstance (Variables|Default|GetCube) 0 0 "None" :!class /Script/Engine.PrimitiveComponent))
  (Variables|Default|SetDinamicMaterial _returnvalue))

(fn ConstructionScript)

(fn BillboardUpdate
  (return (Math|Rotator|FindLookatRotation (Transformation|GetWorldLocation (Variables|Default|GetTextRender)) (Camera|GetCameraLocation (Game|GetPlayerCameraManager 0)))))