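; VR pawn that selects editable objects through a camera-forward line trace and resizes them with a spawned BP_Gizmo.
; Hit actors are classified by interface: Tick tracks the looked-at object, while IA_Interact shows the gizmo, grabs an axis or clears the selection.
; While held on an axis, Tick steps that scale by the sign of hit movement projected onto it and refits the gizmo.
; Gaze fuse and reticle progress helpers exist but are never called here.
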(event EventBeginPlay
  (bind _returnvalue (Game|GetPlayerController 0))
  (Class|HeadMountedDisplayFunctionLibrary|SetTrackingOrigin "Floor")
  (Transformation|SetRelativeLocation (Variables|Default|GetVRCamera) (Variables|Default|GetCamera%20Height) false false)
  (if (Variables|Default|GetEnableMouseHandlers)
    ;[1 1 1] Habilita los click del raton y permite que se muestre en la preview
    (Variables|/Script/Engine.PlayerController|SetbEnableClickEvents _returnvalue true)
    (Variables|/Script/Engine.PlayerController|SetbShowMouseCursor _returnvalue true)))

(event Collision|EventActorBeginOverlap
  (params (OtherActor :type Actor%20Object%20Reference)))

(event EventTick
  (params (DeltaSeconds :type Float%20%28single-precision%29))
  (bind (_returnstart _returnend) (CallFunction|GetStartEndLineTrace))
  (Utilities|FlowControl|Sequence
    (:then_0
      (bind _outhit (Collision|LineTraceByChannel _returnstart _returnend "TraceTypeQuery1" false 0 (select (Variables|Default|GetShowRayCastingLaser) "ForOneFrame" "None")))
      ;[1 1 1] Sirve para filtrar objetos que implementan una interfaz y asi poder definir comportamientos distitos entre ellos
      (bind _interactiontype (CallFunction|GetTargetInteractionType (.hitactor _outhit)))
      (switch Utilities|FlowControl|Switch|SwitchonE_InteractionType _interactiontype
        (:NewEnumerator3
          _)
        (:NewEnumerator4
          _))
      (if (Variables|Default|GetisButtonPressed)
        (if (Variables|Default|GetisDragging)
          (switch Utilities|FlowControl|Switch|SwitchonE_Ejes (Variables|Default|GetEjeActivo)
            (:NewEnumerator1
              (CallFunction|ResizeXAxis (.location _outhit)))
            (:NewEnumerator2
              (CallFunction|ResizeYAxis (.location _outhit)))
            (:NewEnumerator3
              (CallFunction|ResizeZAxis (.location _outhit))))
          (else
            (Development|PrintString "CLICK + No DRAGGING")))
        (elif (not (== (.hitactor _outhit) (Variables|Default|GetTargetedObject)))
          (Variables|Default|SetTargetedObject (.hitactor _outhit))
          (Development|PrintString "nuevo objeto marcado"))))))

(event Input|ActionEvents|InputActionIA_Interact
  (params (Key :type Key%20Structure :default "None"))
  (bind (_returnstart _returnend) (CallFunction|GetStartEndLineTrace))
  (:Pressed
    (Variables|Default|SetisButtonPressed true)
    (Development|PrintString "CLICK BUTTON")
    (bind _outhit (Collision|LineTraceByChannel _returnstart _returnend "TraceTypeQuery1" false 0 "None"))
    ;[1 1 1] Sirve para filtrar objetos que implementan una interfaz y asi poder definir comportamientos distitos entre ellos
    (bind _interactiontype (CallFunction|GetTargetInteractionType (.hitactor _outhit)))
    (switch Utilities|FlowControl|Switch|SwitchonE_InteractionType _interactiontype
      (:NewEnumerator0
        ;[1 1 1] El objeto clickado NO es editable, se limpia todo
        (Class|BPIClickInteraction|OnGazeExit(Message) (Variables|Default|GetCurrentTarget) :!label _label)
        (Variables|Default|SetisDragging false)
        (Variables|Default|SetCurrentTarget 0)
        (Actor|DestroyActor (Variables|Default|GetCurrentGizmo))
        (Development|PrintString "Objeto no editable, limpiando todo"))
      (:NewEnumerator3
        (if (== (.hitactor _outhit) (Variables|Default|GetTargetedObject))
          (if (== (.hitactor _outhit) (Variables|Default|GetCurrentTarget))
            (CallFunction|ShowGizmo (.hitactor _outhit)) ; Marca el objeto como editable muestra el Gizmo y guarda las variables currentTarject y currentGizmo
          )
          (else
            (Development|PrintString "objeto editable DISTINTO")
            (goto _label))))
      (:NewEnumerator4
        ;[1 1 1] Se ha clickado en eje de un gizmo, se guarda el eje clickado y el punto del click ademas de marcarse como Arrastrable
        (bind _ejeselected (Class|BPIGizmoControl|OnAxisPressed(Message) (.hitactor _outhit) (.hitcomponent _outhit)))
        (bind _output_get (Variables|Default|SetEjeActivo _ejeselected))
        (Variables|Default|SetPuntoImpactoInicial (.location _outhit))
        (Variables|Default|SetisDragging true)
        (Variables|Default|SetPantallaInicioClick (.ScreenPosition (Class|GameplayStatics|ProjectWorldtoScreen (Game|GetPlayerController 0) (.location _outhit) false)))
        (Development|PrintString (Utilities|String|EnumtoString _output_get)))))
  (:Released
    (Variables|Default|SetisButtonPressed false)
    (Development|PrintString "DES-CLICK BUTTON")))

(event Input|AxisEvents|InputAxisGiroH
  (params (AxisValue :type Float%20%28single-precision%29))
  (Pawn|Input|AddControllerYawInput AxisValue))

(event Input|AxisEvents|InputAxisGiroV
  (params (AxisValue :type Float%20%28single-precision%29))
  (Pawn|Input|AddControllerPitchInput AxisValue))

(fn ConstructionScript)

(fn GetStartEndLineTrace
  (bind _vrcamera (Variables|Default|GetVRCamera))
  (bind _returnvalue (Transformation|GetWorldLocation _vrcamera))
  (return _returnvalue (+ _returnvalue (* (Math|Vector|GetForwardVector _vrcamera) 1e+03))))

(fn UpdateProgressBar
  (params (Hidden :type Boolean))
  (bind _aswbp_reticle (Utilities|Casting|CastToWBP_Reticle (UserInterface|GetUserWidgetObject (Variables|Default|GetReticleWidget))))
  ;[1 1 1] Actualiza la Progress Bar circular custom
  (Utilities|IsValid (Variables|/Game/UI/WBP_Reticle.WBP_Reticle_C|GetMaterialDynamicRef _aswbp_reticle)
    (:Is%20Valid
      (if Hidden
        (Rendering|Material|SetScalarParameterValue (Variables|/Game/UI/WBP_Reticle.WBP_Reticle_C|GetMaterialDynamicRef _aswbp_reticle) "PercentComplete" 0.0 :!class /Script/Engine.MaterialInstanceDynamic)
        (else
          (Rendering|Material|SetScalarParameterValue (Variables|/Game/UI/WBP_Reticle.WBP_Reticle_C|GetMaterialDynamicRef _aswbp_reticle) "PercentComplete" (/ (Variables|Default|GetCurrentFuseTime) (Variables|Default|GetMaxFuseTime)) :!class /Script/Engine.MaterialInstanceDynamic))))))

(fn GetTargetInteractionType
  (params (TargetActor :type Object%20Object%20Reference))
  (Utilities|FlowControl|Sequence
    (:then_0
      (if (Utilities|DoesObjectImplementInterface TargetActor "/Game/Blueprints/Interfaces/BPI_Interaction.BPI_Interaction_C")
        (return "NewEnumerator1")))
    (:then_1
      (if (Utilities|DoesObjectImplementInterface TargetActor "/Game/Blueprints/Interfaces/BPI_GazeInteraction.BPI_GazeInteraction_C")
        (return "NewEnumerator2")))
    (:then_2
      (if (Utilities|DoesObjectImplementInterface TargetActor "/Game/Blueprints/Interfaces/BPI_ClickInteraction.BPI_ClickInteraction_C")
        (return "NewEnumerator3")))
    (:then_3
      (if (Utilities|DoesObjectImplementInterface TargetActor "/Game/Blueprints/Interfaces/BPI_GizmoControl.BPI_GizmoControl_C")
        (return "NewEnumerator4")))
    (:then_4
      (return "NewEnumerator0"))))

(fn HandleFuseButton
  (bind _output_get (Variables|Default|SetCurrentFuseTime (+ (Variables|Default|GetCurrentFuseTime) (Utilities|Time|GetWorldDeltaSeconds))))
  (if (>= _output_get (Variables|Default|GetMaxFuseTime))
    (Utilities|FlowControl|Sequence
      (:then_0
        ;[1 1 1] Se envia el mensaje a la funcion de la interfaz (si no la tiene no hace nada)
        (Class|BPIInteraction|OnFuseTriggered(Message) (Variables|Default|GetCurrentTarget)))
      (:then_1
        ;[1 1 1] Se resetea el tiempo acumulado
        (Variables|Default|SetCurrentFuseTime 0.0)
        (Development|PrintString "Disparo FUSE BUTTON")
        (return false)))))

(fn ResizeXAxis
  (params (HitLocation :type Vector))
  (bind _currenttarget (Variables|Default|GetCurrentTarget))
  (bind _returnvalue (Transformation|GetActorScale3D _currenttarget))
  (bind (_x _y _z) (Math|Vector|BreakVector _returnvalue))
  (Transformation|SetActorScale3D _currenttarget (Math|Vector|MakeVector (Math|Float|Max(Float) (+ _x (* 0.01 (Math|Float|Sign(Float) (Math|Vector|DotProduct (- HitLocation (Variables|Default|GetPuntoImpactoInicial)) (Math|Vector|GetRightVector (Variables|/Game/Blueprints/Blueprints/BP_Gizmo.BP_Gizmo_C|GetRef_EjeX (Variables|Default|GetCurrentGizmo))))))) 0.05) _y _z))
  ;[1 1 1] Ajustar tamanio gizmo
  (Default|AjustarEjesAlTamano (Variables|Default|GetCurrentGizmo) (Variables|Default|GetCurrentTarget) (Transformation|GetWorldLocation (Variables|Default|GetVRCamera)))
  (return false))

(fn ResizeYAxis
  (params (HitLocation :type Vector))
  (bind _currenttarget (Variables|Default|GetCurrentTarget))
  (bind _returnvalue (Transformation|GetActorScale3D _currenttarget))
  (bind (_x _y _z) (Math|Vector|BreakVector _returnvalue))
  (Transformation|SetActorScale3D _currenttarget (Math|Vector|MakeVector _x (Math|Float|Max(Float) (+ _y (* 0.01 (Math|Float|Sign(Float) (Math|Vector|DotProduct (- HitLocation (Variables|Default|GetPuntoImpactoInicial)) (Math|Vector|GetUpVector (Variables|/Game/Blueprints/Blueprints/BP_Gizmo.BP_Gizmo_C|GetRef_EjeY (Variables|Default|GetCurrentGizmo))))))) 0.05) _z))
  ;[1 1 1] Ajustar tamanio gizmo
  (Default|AjustarEjesAlTamano (Variables|Default|GetCurrentGizmo) (Variables|Default|GetCurrentTarget) (Transformation|GetWorldLocation (Variables|Default|GetVRCamera)))
  (return false))

(fn ResizeZAxis
  (params (HitLocation :type Vector))
  (bind _currenttarget (Variables|Default|GetCurrentTarget))
  (bind _returnvalue (Transformation|GetActorScale3D _currenttarget))
  (bind (_x _y _z) (Math|Vector|BreakVector _returnvalue))
  (Transformation|SetActorScale3D _currenttarget (Math|Vector|MakeVector _x _y (Math|Float|Max(Float) (+ _z (* 0.01 (Math|Float|Sign(Float) (Math|Vector|DotProduct (- HitLocation (Variables|Default|GetPuntoImpactoInicial)) (Math|Vector|GetForwardVector (Variables|/Game/Blueprints/Blueprints/BP_Gizmo.BP_Gizmo_C|GetRef_EjeZ (Variables|Default|GetCurrentGizmo))))))) 0.05)))
  ;[1 1 1] Ajustar tamanio gizmo
  (Default|AjustarEjesAlTamano (Variables|Default|GetCurrentGizmo) (Variables|Default|GetCurrentTarget) (Transformation|GetWorldLocation (Variables|Default|GetVRCamera)))
  (return false))

(fn ShowGizmo
  (params (Current%20Target :type Actor%20Object%20Reference))
  (bind _output_get (Variables|Default|SetCurrentTarget Current%20Target))
  (Class|BPIClickInteraction|OnDirectClick(Message) _output_get "0, 0, 0") ; Cambia el color del objeto
  ;[1 1 1] Se muestra y ajusta el Gizmo y se adjunta al objeto editable
  (bind _returnvalue (Game|SpawnActorfromClass "/Game/Blueprints/Blueprints/BP_Gizmo.BP_Gizmo_C" (Math|Transform|MakeTransform (Transformation|GetActorLocation _output_get) "0, 0, 0" "1,1,1") "Undefined" 0 0))
  (bind _output_get_2 (Variables|Default|SetCurrentGizmo _returnvalue))
  (Default|AjustarEjesAlTamano _output_get_2 _output_get (Transformation|GetWorldLocation (Variables|Default|GetVRCamera)))
  (Transformation|AttachActorToActor _output_get_2 _output_get "None" "SnapToTarget" "KeepRelative" "KeepRelative" true)
  (return false))