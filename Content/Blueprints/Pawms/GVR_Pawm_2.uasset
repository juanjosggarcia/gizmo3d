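; VR pawn for gaze interaction, with camera look driven by gyro-named axis inputs and optional mouse click support.
; Each tick it traces from the camera and classifies the hit actor by interface, sending hover, exit or gizmo-axis messages.
; Dwelling on Interactive targets fills a circular reticle and fires a fuse event.
; IA_Interact direct-clicks the target, pauses its fuse and attaches a new BP_Gizmo; Gaze-only and Click-only types are unhandled.
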(event EventBeginPlay
  (bind _returnvalue (Game|GetPlayerController 0))
  (Class|HeadMountedDisplayFunctionLibrary|SetTrackingOrigin "Floor")
  (Transformation|SetRelativeLocation (Variables|Default|GetVRCamera) (Variables|Default|GetCamera%20Height) false false)
  (if (Variables|Default|GetEnableMouseHandlers)
    ;[1 1 1] Habilita los click del raton y permite que se muestre en la preview
    (Variables|/Script/Engine.PlayerController|SetbEnableClickEvents _returnvalue true)
    (Variables|/Script/Engine.PlayerController|SetbShowMouseCursor _returnvalue true)))

(event Collision|EventActorBeginOverlap
  (params (OtherActor :type Actor%20Object%20Reference)))

(event EventTick
  (params (DeltaSeconds :type Float%20%28single-precision%29))
  (bind (_returnstart _returnend) (CallFunction|GetStartEndLineTrace))
  (Utilities|FlowControl|Sequence
    (:then_0
      (bind _outhit (Collision|LineTraceByChannel _returnstart _returnend "TraceTypeQuery1" false 0 (select (Variables|Default|GetShowRayCastingLaser) "ForOneFrame" "None")))
      ;[1 1 1] Sirve para filtrat objetos que implementan una interfaz y asi poder definir comportamientos distitos entre ellos
      (bind _interactiontype (CallFunction|GetTargetInteractionType (.hitactor _outhit)))
      (switch Utilities|FlowControl|Switch|SwitchonE_InteractionType _interactiontype
        (:NewEnumerator0
          ;[1 1 1] El Objeto ya no es valido, Limpia el color (en caso necesitarlo), se nulea y se reinicia el tiempo acumulado
          (Class|BPIInteraction|OnGazeExit(Message) (Variables|Default|GetCurrentTarget))
          (Variables|Default|SetisButtonPressed false)
          (Variables|Default|SetCurrentTarget 0)
          (Variables|Default|SetCurrentFuseTime 0.0 :!label _label))
        (:NewEnumerator1
          (if (not (Variables|Default|GetisButtonPressed))
            (Class|BPIInteraction|OnGazeHover(Message) (Variables|Default|GetCurrentTarget))
            ;[1 1 1] Se comprueba si NO se ha quitado la vista del objeto selecionado o si es la primera vez que se ha visto el objeto
            (if (== (Variables|Default|GetCurrentTarget) (.hitactor _outhit))
              (CallFunction|HandleFuseButton)
              (else
                ;[1 1 1] Primera vez que se mira el objeto, se limpia y guarda el objeto
                (Class|BPIInteraction|OnGazeExit(Message) (Variables|Default|GetCurrentTarget))
                (Variables|Default|SetCurrentTarget (.hitactor _outhit))
                (goto _label)))))
        (:NewEnumerator4
          (bind _ejeselected (Class|BPIGizmoControl|OnAxisPressed(Message) (.hitactor _outhit) (.hitcomponent _outhit)))
          (Development|PrintString (Utilities|String|EnumtoString _ejeselected)))))
    (:then_1
      (CallFunction|UpdateProgressBar (Variables|Default|GetisButtonPressed)))))

(event Input|ActionEvents|InputActionIA_Interact
  (params (Key :type Key%20Structure :default "None"))
  (bind _currenttarget (Variables|Default|GetCurrentTarget))
  (:Pressed
    (Development|PrintString "CLICK BUTTON")
    ;[1 1 1] Sirve para filtrat objetos que implementan una interfaz y asi poder definir comportamientos distitos entre ellos
    (bind _interactiontype (CallFunction|GetTargetInteractionType _currenttarget))
    (switch Utilities|FlowControl|Switch|SwitchonE_InteractionType _interactiontype
      (:NewEnumerator1
        ;[1 1 1] Se envia el mensaje a la funcion de la interfaz (si no la tiene no hace nada)
        (Class|BPIInteraction|OnDirectClick(Message) _currenttarget)
        (Variables|Default|SetisButtonPressed true)
        (Development|PrintString "Disparo CLICK BUTTON + GAZE")
        (bind _returnvalue (Game|SpawnActorfromClass "/Game/Blueprints/Blueprints/BP_Gizmo.BP_Gizmo_C" (Math|Transform|MakeTransform (Transformation|GetActorLocation _currenttarget) "0, 0, 0" "1,1,1") "Undefined" 0 0))
        (bind _output_get (Variables|Default|SetCurrentGizmo _returnvalue))
        (Transformation|AttachActorToActor _output_get _currenttarget "None" "SnapToTarget" "KeepRelative" "KeepRelative" true)
        (Default|AjustarEjesAlTamano (Variables|Default|GetCurrentGizmo) 0 "0, 0, 0")
        (Development|PrintString "Selecionado cubo para moverlo")))))

(event Input|AxisEvents|InputAxisGiroH
  (params (AxisValue :type Float%20%28single-precision%29))
  (Pawn|Input|AddControllerYawInput AxisValue))

(event Input|AxisEvents|InputAxisGiroV
  (params (AxisValue :type Float%20%28single-precision%29))
  (Pawn|Input|AddControllerPitchInput AxisValue))

(fn ConstructionScript)

(fn GetStartEndLineTrace
  (bind _vrcamera (Variables|Default|GetVRCamera))
  (bind _returnvalue (Transformation|GetWorldLocation _vrcamera))
  (return _returnvalue (+ _returnvalue (* (Math|Vector|GetForwardVector _vrcamera) 1e+03))))

(fn UpdateProgressBar
  (params (Hidden :type Boolean))
  (bind _aswbp_reticle (Utilities|Casting|CastToWBP_Reticle (UserInterface|GetUserWidgetObject (Variables|Default|GetReticleWidget))))
  ;[1 1 1] Actualiza la Progress Bar circular custom
  (Utilities|IsValid (Variables|/Game/UI/WBP_Reticle.WBP_Reticle_C|GetMaterialDynamicRef _aswbp_reticle)
    (:Is%20Valid
      (if Hidden
        (Rendering|Material|SetScalarParameterValue (Variables|/Game/UI/WBP_Reticle.WBP_Reticle_C|GetMaterialDynamicRef _aswbp_reticle) "PercentComplete" 0.0 :!class /Script/Engine.MaterialInstanceDynamic)
        (else
          (Rendering|Material|SetScalarParameterValue (Variables|/Game/UI/WBP_Reticle.WBP_Reticle_C|GetMaterialDynamicRef _aswbp_reticle) "PercentComplete" (/ (Variables|Default|GetCurrentFuseTime) (Variables|Default|GetMaxFuseTime)) :!class /Script/Engine.MaterialInstanceDynamic))))))

(fn GetTargetInteractionType
  (params (TargetActor :type Object%20Object%20Reference))
  (Utilities|FlowControl|Sequence
    (:then_0
      (if (Utilities|DoesObjectImplementInterface TargetActor "/Game/Blueprints/Interfaces/BPI_Interaction.BPI_Interaction_C")
        (return "NewEnumerator1")))
    (:then_1
      (if (Utilities|DoesObjectImplementInterface TargetActor "/Game/Blueprints/Interfaces/BPI_GazeInteraction.BPI_GazeInteraction_C")
        (return "NewEnumerator2")))
    (:then_2
      (if (Utilities|DoesObjectImplementInterface TargetActor "/Game/Blueprints/Interfaces/BPI_ClickInteraction.BPI_ClickInteraction_C")
        (return "NewEnumerator3")))
    (:then_3
      (if (Utilities|DoesObjectImplementInterface TargetActor "/Game/Blueprints/Interfaces/BPI_GizmoControl.BPI_GizmoControl_C")
        (return "NewEnumerator4")))
    (:then_4
      (return "NewEnumerator0"))))

(fn HandleFuseButton
  (bind _output_get (Variables|Default|SetCurrentFuseTime (+ (Variables|Default|GetCurrentFuseTime) (Utilities|Time|GetWorldDeltaSeconds))))
  (if (>= _output_get (Variables|Default|GetMaxFuseTime))
    (Utilities|FlowControl|Sequence
      (:then_0
        ;[1 1 1] Se envia el mensaje a la funcion de la interfaz (si no la tiene no hace nada)
        (Class|BPIInteraction|OnFuseTriggered(Message) (Variables|Default|GetCurrentTarget)))
      (:then_1
        ;[1 1 1] Se resetea el tiempo acumulado
        (Variables|Default|SetCurrentFuseTime 0.0)
        (Development|PrintString "Disparo FUSE BUTTON")
        (return false)))))