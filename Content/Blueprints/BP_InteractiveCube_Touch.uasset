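; BP_InteractiveCube_Touch is an interactive cube that turns red while a GVR_Pawm actor overlaps it.
; BeginPlay creates a dynamic material on the Cube.
; Its overlap events set an IsHandOverlapping flag and switch ColorParam to red, then back to white on exit.
; A BillboardUpdate helper computes a camera-facing rotation for the TextRender, but the call applying it is unconnected, so the text never turns.
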(event OnComponentBeginOverlap(Cube)
  (params (OverlappedComponent :type Primitive%20Component%20Object%20Reference) (OtherActor :type Actor%20Object%20Reference) (OtherComp :type Primitive%20Component%20Object%20Reference) (OtherBodyIndex :type Integer) (bFromSweep :type Boolean) (SweepResult :type Hit%20Result%20Structure%20%28by%20ref%29))
  (Utilities|Casting|CastToGVR_Pawm OtherActor)
  (Variables|Default|SetisHandOverlapping true)
  (Rendering|Material|SetVectorParameterValue (Variables|Default|GetDinamicMaterial) "ColorParam" "(R=1.000000,G=0.000000,B=0.000000,A=1.000000)" :!class /Script/Engine.MaterialInstanceDynamic))

(event OnComponentEndOverlap(Cube)
  (params (OverlappedComponent :type Primitive%20Component%20Object%20Reference) (OtherActor :type Actor%20Object%20Reference) (OtherComp :type Primitive%20Component%20Object%20Reference) (OtherBodyIndex :type Integer))
  (Utilities|Casting|CastToGVR_Pawm OtherActor)
  (Variables|Default|SetisHandOverlapping false)
  (Rendering|Material|SetVectorParameterValue (Variables|Default|GetDinamicMaterial) "ColorParam" "(R=1.000000,G=1.000000,B=1.000000,A=1.000000)" :!class /Script/Engine.MaterialInstanceDynamic))

(event Collision|EventActorBeginOverlap
  (params (OtherActor :type Actor%20Object%20Reference)))

(event EventTick
  (params (DeltaSeconds :type Float%20%28single-precision%29)))

(event EventBeginPlay
  (bind _returnvalue (Rendering|Material|CreateDynamicMaterialInstance (Variables|Default|GetCube) 0 0 "None" :!class /Script/Engine.PrimitiveComponent))
  (Variables|Default|SetDinamicMaterial _returnvalue))

(fn ConstructionScript)

(fn BillboardUpdate
  (return (Math|Rotator|FindLookatRotation (Transformation|GetWorldLocation (Variables|Default|GetTextRender)) (Camera|GetCameraLocation (Game|GetPlayerCameraManager 0)))))