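; BP_Gizmo is a gizmo actor with X, Y and Z axis cylinders that can be fitted to the size of a parent.
; AjustarEjesAlTamano takes the parent's size and moves each cylinder along its own axis to that dimension plus a small fixed margin.
; It only changes relative locations, with no scaling.
; The event graph and construction script are empty, so the function relies on an external caller.
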(event EventBeginPlay)

(event Collision|EventActorBeginOverlap
  (params (OtherActor :type Actor%20Object%20Reference)))

(event EventTick
  (params (DeltaSeconds :type Float%20%28single-precision%29)))

(fn ConstructionScript)

(fn AjustarEjesAlTamano
  (params (TamanoPadre :type Vector))
  (bind (_x _y _z) (Math|Vector|BreakVector TamanoPadre))
  (Utilities|FlowControl|Sequence
    (:then_0
      (Transformation|SetRelativeLocation (Variables|Default|GetEjeX_Cilindro) (Math|Vector|MakeVector (+ _x 5.0) 0.0 0.0) false false))
    (:then_1
      (Transformation|SetRelativeLocation (Variables|Default|GetEjeY_Cilindro) (Math|Vector|MakeVector 0.0 (+ _y 5.0) 0.0) false false))
    (:then_2
      (Transformation|SetRelativeLocation (Variables|Default|GetEjeZ_Cilindro) (Math|Vector|MakeVector 0.0 0.0 (+ _z 5.0)) false false))))