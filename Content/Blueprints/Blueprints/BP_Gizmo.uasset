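; BP_Gizmo is a three-axis transform gizmo with cylinder, cone and rotate handles for manipulating a target actor.
; BeginPlay maps each handle component to an axis/action SGizmoHitData, which OnAxisPressed looks up, returning a default pair for unknown components.
; AjustarEjesAlTamano scales the axis cylinders to the target's colliding bounds; its camera input only feeds dead code.
; GetAction is a stub returning the same enum value on every returning path.
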(event EventBeginPlay
  (bind _ejex_cilindro (Variables|Default|GetEjeX_Cilindro))
  (bind _ejey_cilindro (Variables|Default|GetEjeY_Cilindro))
  (bind _rotateejex_top (Variables|Default|GetRotateEjeX_Top))
  (bind _rotateejex_bottom (Variables|Default|GetRotateEjeX_Bottom))
  (bind _rotateejey_top (Variables|Default|GetRotateEjeY_Top))
  (bind _rotateejey_bottom (Variables|Default|GetRotateEjeY_Bottom))
  (bind _rotateejez_bottom (Variables|Default|GetRotateEjeZ_Bottom))
  (bind _rotateejez_top (Variables|Default|GetRotateEjeZ_Top))
  (bind _ejez_cilindro (Variables|Default|GetEjeZ_Cilindro))
  (bind _mapa_gizmo (Variables|Default|GetMapa_Gizmo))
  (bind _ejextop_cone (Variables|Default|GetEjeXTop_Cone))
  (bind _ejexbottom_cone (Variables|Default|GetEjeXBottom_Cone))
  (bind _ejeytop_cone (Variables|Default|GetEjeYTop_Cone))
  (bind _ejeybuttom_cone (Variables|Default|GetEjeYButtom_Cone))
  (bind _ejeztop_cone (Variables|Default|GetEjeZTop_Cone))
  (bind _ejezbottom_cone (Variables|Default|GetEjeZBottom_Cone))
  (Utilities|FlowControl|Sequence
    (:then_0
      (Utilities|Map|Add _mapa_gizmo _ejex_cilindro (Utilities|Struct|MakeS_GizmoHitData "NewEnumerator1" "NewEnumerator0"))
      (Utilities|Map|Add _mapa_gizmo _ejey_cilindro (Utilities|Struct|MakeS_GizmoHitData "NewEnumerator2" "NewEnumerator0"))
      (Utilities|Map|Add _mapa_gizmo _ejez_cilindro (Utilities|Struct|MakeS_GizmoHitData "NewEnumerator3" "NewEnumerator0"))
      (Utilities|Map|Add _mapa_gizmo _ejextop_cone (Utilities|Struct|MakeS_GizmoHitData "NewEnumerator1" "NewEnumerator1"))
      (Utilities|Map|Add _mapa_gizmo _ejexbottom_cone (Utilities|Struct|MakeS_GizmoHitData "NewEnumerator1" "NewEnumerator1"))
      (Utilities|Map|Add _mapa_gizmo _ejeytop_cone (Utilities|Struct|MakeS_GizmoHitData "NewEnumerator2" "NewEnumerator1"))
      (Utilities|Map|Add _mapa_gizmo _ejeybuttom_cone (Utilities|Struct|MakeS_GizmoHitData "NewEnumerator2" "NewEnumerator1"))
      (Utilities|Map|Add _mapa_gizmo _ejeztop_cone (Utilities|Struct|MakeS_GizmoHitData "NewEnumerator3" "NewEnumerator1"))
      (Utilities|Map|Add _mapa_gizmo _ejezbottom_cone (Utilities|Struct|MakeS_GizmoHitData "NewEnumerator3" "NewEnumerator1"))
      (Utilities|Map|Add _mapa_gizmo _rotateejex_top (Utilities|Struct|MakeS_GizmoHitData "NewEnumerator1" "NewEnumerator2"))
      (Utilities|Map|Add _mapa_gizmo _rotateejex_bottom (Utilities|Struct|MakeS_GizmoHitData "NewEnumerator1" "NewEnumerator2"))
      (Utilities|Map|Add _mapa_gizmo _rotateejey_top (Utilities|Struct|MakeS_GizmoHitData "NewEnumerator2" "NewEnumerator2"))
      (Utilities|Map|Add _mapa_gizmo _rotateejey_bottom (Utilities|Struct|MakeS_GizmoHitData "NewEnumerator2" "NewEnumerator2"))
      (Utilities|Map|Add _mapa_gizmo _rotateejez_top (Utilities|Struct|MakeS_GizmoHitData "NewEnumerator3" "NewEnumerator2"))
      (Utilities|Map|Add _mapa_gizmo _rotateejez_bottom (Utilities|Struct|MakeS_GizmoHitData "NewEnumerator3" "NewEnumerator2")))
    (:then_1
      (Variables|Default|SetRef_EjeX _ejex_cilindro)
      (Variables|Default|SetRef_EjeY _ejey_cilindro)
      (Variables|Default|SetRef_EjeZ _ejez_cilindro)
      (Variables|Default|SetRef_EjeX_Top _ejextop_cone)
      (Variables|Default|SetRef_EjeX_Buttom _ejexbottom_cone)
      (Variables|Default|SetRef_EjeY_Top _ejeytop_cone)
      (Variables|Default|SetRef_EjeY_Buttom _ejeybuttom_cone)
      (Variables|Default|SetRef_EjeZ_Top _ejeztop_cone)
      (Variables|Default|SetRef_EjeZ_Buttom _ejezbottom_cone)
      (Variables|Default|SetRef_RotateX_Top _rotateejex_top)
      (Variables|Default|SetRef_RotateX_Bottom _rotateejex_bottom)
      (Variables|Default|SetRef_RotateY_Top _rotateejey_top)
      (Variables|Default|SetRef_RotateY_Bottom _rotateejey_bottom)
      (Variables|Default|SetRef_RotateZ_Top _rotateejez_top)
      (Variables|Default|SetRef_RotateZ_Bottom _rotateejez_bottom))))

(event Collision|EventActorBeginOverlap
  (params (OtherActor :type Actor%20Object%20Reference)))

(event EventTick
  (params (DeltaSeconds :type Float%20%28single-precision%29)))

(fn ConstructionScript)

(fn AjustarEjesAlTamano
  (params (ActorObjetivo :type Actor%20Object%20Reference) (UbicacionCamara :type Vector))
  (bind _boxextent (Collision|GetActorBounds ActorObjetivo true false))
  (bind _ejex_cilindro (Variables|Default|GetEjeX_Cilindro))
  (bind _ejey_cilindro (Variables|Default|GetEjeY_Cilindro))
  (bind _ejez_cilindro (Variables|Default|GetEjeZ_Cilindro))
  (bind (_x _y _z) (Math|Vector|BreakVector _boxextent))
  (Utilities|FlowControl|Sequence
    (:then_0
      ;[1 1 1] Logica Eje X
      (Transformation|SetRelativeScale3D _ejex_cilindro (Math|Vector|MakeVector 0.07 0.07 (/ (* _x 2.8) 1e+02)))
      (Transformation|SetRelativeLocation _ejex_cilindro (Math|Vector|MakeVector 0.0 0.0 0.0) false false))
    (:then_1
      ;[1 1 1] Logica Eje Y
      (Transformation|SetRelativeScale3D _ejey_cilindro (Math|Vector|MakeVector 0.07 0.07 (/ (* _y 2.8) 1e+02)))
      (Transformation|SetRelativeLocation _ejey_cilindro (Math|Vector|MakeVector 0.0 0.0 0.0) false false))
    (:then_2
      ;[1 1 1] Logica Eje Z
      (Transformation|SetRelativeScale3D _ejez_cilindro (Math|Vector|MakeVector 0.07 0.07 (/ (* _z 2.8) 1e+02)))
      (Transformation|SetRelativeLocation _ejez_cilindro (Math|Vector|MakeVector 0.0 0.0 0.0) false false))))

(fn GetAction
  (params (Component :type Actor%20Component%20Object%20Reference))
  (Utilities|FlowControl|Sequence
    (:then_0
      (if (== (Variables|Default|GetRef_EjeX_Top) Component)
        (return "NewEnumerator0")
        (elif (== (Variables|Default|GetRef_EjeX_Buttom) Component)
          (return "NewEnumerator0"))))
    (:then_1
      (if (== Component (Variables|Default|GetRef_EjeY_Top))
        (return "NewEnumerator0")
        (elif (== Component (Variables|Default|GetRef_EjeY_Buttom))
          (return "NewEnumerator0"))))
    (:then_2
      (if (== Component (Variables|Default|GetRef_EjeZ_Top))
        (return "NewEnumerator0")
        (elif (== Component (Variables|Default|GetRef_EjeZ_Buttom))
          (return "NewEnumerator0"))))
    (:then_3
      (return "NewEnumerator0"))))

(fn OnAxisPressed
  (params (Componente :type Actor%20Component%20Object%20Reference))
  (bind _mapa_gizmo (Variables|Default|GetMapa_Gizmo))
  (bind (_value _returnvalue) (Utilities|Map|Find _mapa_gizmo Componente))
  (if _returnvalue
    (return _value)
    (else
      (return (Utilities|Struct|MakeS_GizmoHitData "NewEnumerator0" "NewEnumerator3")))))