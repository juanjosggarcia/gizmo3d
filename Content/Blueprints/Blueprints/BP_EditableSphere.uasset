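; BP_EditableSphere is an interactive sphere actor that highlights in cyan when clicked and returns to white when gaze leaves it.
; BeginPlay creates a dynamic material instance on the sphere, and the click, direct-click and gaze-exit events set its ColorParam.
; A BillboardUpdate function computes a rotation from the text render toward the player camera, but the node applying it is never run.
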(event Collision|EventActorBeginOverlap
  (params (OtherActor :type Actor%20Object%20Reference)))

(event EventTick
  (params (DeltaSeconds :type Float%20%28single-precision%29)))

(event EventOnGazeExit
  (Rendering|Material|SetVectorParameterValue (Variables|Default|GetDinamicMaterial) "ColorParam" "(R=1.000000,G=1.000000,B=1.000000,A=1.000000)" :!class /Script/Engine.MaterialInstanceDynamic))

(event EventBeginPlay
  (bind _returnvalue (Rendering|Material|CreateDynamicMaterialInstance (Variables|Default|GetSphere) 0 0 "None" :!class /Script/Engine.PrimitiveComponent))
  (Variables|Default|SetDinamicMaterial _returnvalue))

(event MouseInput|EventActorOnClicked
  (params (ButtonPressed :type Key%20Structure :default "None"))
  (Rendering|Material|SetVectorParameterValue (Variables|Default|GetDinamicMaterial) "ColorParam" "(R=0.000000,G=1.000000,B=1.000000,A=1.000000)" :!class /Script/Engine.MaterialInstanceDynamic))

(event EventOnDirectClick
  (params (clickLocation :type Vector :default "0, 0, 0"))
  (Rendering|Material|SetVectorParameterValue (Variables|Default|GetDinamicMaterial) "ColorParam" "(R=0.000000,G=1.000000,B=1.000000,A=1.000000)" :!class /Script/Engine.MaterialInstanceDynamic))

(fn ConstructionScript)

(fn BillboardUpdate
  (return (Math|Rotator|FindLookatRotation (Transformation|GetWorldLocation (Variables|Default|GetTextRender)) (Camera|GetCameraLocation (Game|GetPlayerCameraManager 0)))))